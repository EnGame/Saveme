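; Hero_BP is a player-controlled character with movement, mouse look, sprint and jump driven by input events.
; Movement axes add input along the Camera's forward and right vectors and play the Hero_HeadShake camera shake on player 0, scaled by the axis value.
; Look axes feed controller pitch and yaw, while Sprint switches CharacterMovement's max walk speed between RunSpeed and WalkSpeed.
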(event Input|ActionEvents|InputActionJump
  (params (Key :type Key%20Structure))
  ;[1 1 1] Jump-Без прыжка не кайф играть
  (:Pressed
    (Character|Jump))
  (:Released
    (Character|StopJumping)))

(event Input|ActionEvents|InputActionSprint
  (params (Key :type Key%20Structure))
  (bind _charactermovement (Variables|Character|GetCharacterMovement))
  ;[1 1 1] Sprint
  (:Pressed
    (Variables|/Script/Engine.CharacterMovementComponent|SetMaxWalkSpeed _charactermovement (Variables|Default|GetRun_speed)))
  (:Released
    (Variables|/Script/Engine.CharacterMovementComponent|SetMaxWalkSpeed _charactermovement (Variables|Default|GetWalk_speed))))

(event Input|AxisEvents|InputAxisMove_forward
  (params (AxisValue :type Float%20%28single-precision%29))
  ;[1 1 1] Movement
  (Pawn|Input|AddMovementInput (Math|Vector|GetForwardVector (Variables|Default|GetCamera)) AxisValue false)
  (Class|PlayerController|ClientPlayCameraShake (Game|GetPlayerController 0) "/Game/Characters/Hero/Hero_HeadShake.Hero_HeadShake_C" AxisValue "CameraLocal" "0, 0, 0"))

(event Input|AxisEvents|InputAxisLeft_strife
  (params (AxisValue :type Float%20%28single-precision%29))
  ;[1 1 1] Movement
  (Pawn|Input|AddMovementInput (Math|Vector|GetRightVector (Variables|Default|GetCamera)) AxisValue false)
  (Class|PlayerController|ClientPlayCameraShake (Game|GetPlayerController 0) "/Game/Characters/Hero/Hero_HeadShake.Hero_HeadShake_C" AxisValue "CameraLocal" "0, 0, 0"))

(event Input|AxisEvents|InputAxisLook_left
  (params (AxisValue :type Float%20%28single-precision%29))
  ;[1 1 1] Mouse Look
  (Pawn|Input|AddControllerYawInput AxisValue))

(event Input|AxisEvents|InputAxisLook_Up
  (params (AxisValue :type Float%20%28single-precision%29))
  ;[1 1 1] Mouse Look
  (Pawn|Input|AddControllerPitchInput AxisValue))

(fn ConstructionScript)